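; VolcanoballGame runs the eruption timer for the Volcanoball game and respawns dead volcanoballs each time the volcano erupts.
; On BeginPlay it fetches the single BP_VolcanoballConstants actor in the level, printing an error unless exactly one exists, and picks a random wait between its minimum and maximum.
; Tick counts that wait down, then picks a new one, calls RespawnMe on every entry in DeadVolcanoballs and clears the list.
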(event `self.ReceiveBeginPlay`
  (bind _constants (`self.Constants`))
  ;[1 1 1] Get the game constants object
  (bind _outactors (`GameplayStatics.GetAllActorsOfClass` "/Game/Blueprints/Volcanoball/BP_VolcanoballConstants.BP_VolcanoballConstants_C"))
  (if (!= (`KismetArrayLibrary.Array_Length` _outactors) 1)
    (`KismetSystemLibrary.PrintString` "ERROR: Must be exactly ONE 'VolcanoballConstants' object in scene!" true true (struct :`R` 1.0 :`A` 1.0))
    (else
      (set `self.Constants` (`KismetArrayLibrary.Array_Get` _outactors))
      ;[1 1 1] Set initial time to erupt
      (set `self.Time To Blow` (`KismetMathLibrary.Lerp` (`/Game/Blueprints/Volcanoball/BP_VolcanoballConstants.Min Volcano Wait Time` _constants) (`/Game/Blueprints/Volcanoball/BP_VolcanoballConstants.Max Volcano Wait Time` _constants) (`KismetMathLibrary.RandomFloat`))))))

(event `self.ReceiveTick`
  (params (DeltaSeconds :type "Float (single-precision)"))
  (bind _constants (`self.Constants`))
  (bind _dead_volcanoballs (`self.Dead Volcanoballs`))
  (set `self.Time To Blow` (- (`self.Time To Blow`) DeltaSeconds))
  (if (<= (`self.Time To Blow`) 0.0)
    (`KismetSystemLibrary.PrintString` "TRIGGER ERUPTION")
    (set `self.Time To Blow` (`KismetMathLibrary.Lerp` (`/Game/Blueprints/Volcanoball/BP_VolcanoballConstants.Min Volcano Wait Time` _constants) (`/Game/Blueprints/Volcanoball/BP_VolcanoballConstants.Max Volcano Wait Time` _constants) (`KismetMathLibrary.RandomFloat`)))
    (for _array_element _dead_volcanoballs
      (`/Game/Blueprints/Volcanoball/BP_VolcanoBall.Respawn Me` _array_element))
    (`KismetArrayLibrary.Array_Clear` _dead_volcanoballs)))

(fn `UserConstructionScript`)