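; Snowball actor that stays hidden and physically asleep for a random delay before appearing in the game.
; On BeginPlay it casts the game mode to SnowballGame and requests a random wait time.
; Tick counts that time down, hiding the actor and putting its rigid body to sleep while time remains, then unhiding and waking it every frame thereafter.
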(event `self.ReceiveBeginPlay`
  ;[1 1 1] Startup
  (bind _assnowball_game (cast `/Game/Blueprints/SnowballGame` (`GameplayStatics.GetGameMode`)))
  (set `self.HideTime` (`/Game/Blueprints/SnowballGame.Get Random Snowball Wait Time` _assnowball_game)))

(event `self.ReceiveTick`
  (params (DeltaSeconds :type "Float (single-precision)"))
  (bind _returnvalue (> (`self.HideTime`) 0.0))
  ;[1 1 1] Tick
  (set `self.HideTime` (- (`self.HideTime`) DeltaSeconds))
  (`self.SetActorHiddenInGame` _returnvalue)
  (if _returnvalue
    (`PrimitiveComponent.PutRigidBodyToSleep` "None")
    (else
      (`PrimitiveComponent.WakeRigidBody` "None"))))

(fn `UserConstructionScript`)