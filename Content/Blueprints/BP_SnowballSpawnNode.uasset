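; BP_SnowballSpawnNode is a placed spawn point that launches snowballs it is given.
; SpawnSnowball moves the passed snowball to the node's location and sets its physics velocity to a random blend between the min and max spawn velocities.
; It then sets the snowball's HideTime from a random wait time supplied by the SnowballGame game mode.
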(fn `Spawn Snowball`
  (params (`Snowball To Spawn` :type "/Game/Blueprints/BP_Snowball Object Reference"))
  (`self.K2_SetActorLocation` `Snowball To Spawn` (`self.K2_GetActorLocation`) false)
  (`PrimitiveComponent.SetPhysicsLinearVelocity` (`/Game/Blueprints/BP_Snowball.Mesh` `Snowball To Spawn`) (`KismetMathLibrary.VLerp` (`self.Min Spawn Velocity`) (`self.Max Spawn Velocity`) (`KismetMathLibrary.RandomFloat`)) false "None")
  (bind _assnowball_game (cast `/Game/Blueprints/SnowballGame` (`GameplayStatics.GetGameMode`)))
  (set `/Game/Blueprints/BP_Snowball.HideTime` (`/Game/Blueprints/SnowballGame.Get Random Snowball Wait Time` _assnowball_game) `Snowball To Spawn`))

(fn `UserConstructionScript`)