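; Physics ball for the Volcanoball game mode, recycled through a dead and respawn cycle instead of being destroyed.
; It starts dead, and also dies after idling at low speed for several seconds, moving far off to a random point and joining the game mode's DeadVolcanoballs.
; Disabled gravity doubles as the dead flag, with Tick cancelling any velocity.
; RespawnMe teleports it to its start and launches it with random velocity within game mode limits.
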(event `self.ReceiveBeginPlay`
  (set `self.Start Position` (`self.K2_GetActorLocation`))
  (`self.Kill Me`))

(event `self.ReceiveTick`
  (params (DeltaSeconds :type "Float (single-precision)"))
  (if (`self.Is Dead?`)
    (`PrimitiveComponent.AddImpulse` (- (0.0 0.0 0.0) (`self.GetVelocity`)) "None" true)
    (elif (< (`KismetMathLibrary.VSize` (`self.GetVelocity`)) 50.0)
      (set `self.Time Idle` (+ DeltaSeconds (`self.Time Idle`)))
      (if (> (`self.Time Idle`) 6.0)
        (`self.Kill Me`))
      (else
        (set `self.Time Idle` 0.0)))))

(fn `Is Dead?`
  (returns (Value :type Boolean))
  (return (not (`PrimitiveComponent.IsGravityEnabled`))))

(fn `Kill Me`
  (set `self.Time Idle` 0.0)
  (`self.K2_SetActorLocation` (`KismetMathLibrary.VLerp` (-9999.0 -99999.0 -9999.0) (99999.0 99999.0 -9999.0) (`KismetMathLibrary.RandomFloat`)))
  (`PrimitiveComponent.SetAllPhysicsLinearVelocity` (0.0 0.0 0.0))
  (`PrimitiveComponent.SetEnableGravity` false)
  (bind _asvolcanoball_game (cast `/Game/Blueprints/Volcanoball/VolcanoballGame` (`GameplayStatics.GetGameMode`)))
  (`KismetArrayLibrary.Array_Add` (`/Game/Blueprints/Volcanoball/VolcanoballGame.Dead Volcanoballs` _asvolcanoball_game) self))

(fn `Respawn Me`
  (`PrimitiveComponent.SetEnableGravity` true)
  (`self.K2_TeleportTo` (`self.Start Position`))
  (bind _asvolcanoball_game (cast `/Game/Blueprints/Volcanoball/VolcanoballGame` (`GameplayStatics.GetGameMode`)))
  (bind _constants (`/Game/Blueprints/Volcanoball/VolcanoballGame.Constants` _asvolcanoball_game))
  (`PrimitiveComponent.AddImpulse` (`KismetMathLibrary.MakeVector` (`KismetMathLibrary.Lerp` (.x (`/Game/Blueprints/Volcanoball/BP_VolcanoballConstants.Min Ball Respawn Velocity` _constants)) (.x (`/Game/Blueprints/Volcanoball/BP_VolcanoballConstants.Max Ball Respawn Velocity` _constants)) (`KismetMathLibrary.RandomFloat`)) (`KismetMathLibrary.Lerp` (.y (`/Game/Blueprints/Volcanoball/BP_VolcanoballConstants.Min Ball Respawn Velocity` _constants)) (.y (`/Game/Blueprints/Volcanoball/BP_VolcanoballConstants.Max Ball Respawn Velocity` _constants)) (`KismetMathLibrary.RandomFloat`)) (`KismetMathLibrary.Lerp` (.z (`/Game/Blueprints/Volcanoball/BP_VolcanoballConstants.Min Ball Respawn Velocity` _constants)) (.z (`/Game/Blueprints/Volcanoball/BP_VolcanoballConstants.Max Ball Respawn Velocity` _constants)) (`KismetMathLibrary.RandomFloat`))) "None" true))

(fn `UserConstructionScript`)