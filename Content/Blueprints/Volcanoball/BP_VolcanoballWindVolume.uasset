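; Wind volume for Volcanoball that pushes volcano balls inside it horizontally along the line out from its origin.
; The collision box's begin overlap adds balls to a tracked array, and the actor's end overlap removes them.
; Each tick applies a Force-scaled, mass-independent velocity-change impulse to every tracked ball, without delta-time scaling, so the push depends on frame rate.
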(event `self.Collision Box.OnComponentBeginOverlap`
  (params (OtherActor :type "Actor Object Reference") (OtherComp :type "PrimitiveComponent Object Reference") (OtherBodyIndex :type Integer) (bFromSweep :type Boolean) (SweepResult :type "EngineTypes.HitResult Structure (by ref)"))
  (bind _asbp_volcano_ball (cast `/Game/Blueprints/Volcanoball/BP_VolcanoBall` OtherActor))
  (`KismetArrayLibrary.Array_Add` (`self.Balls being touched`) _asbp_volcano_ball))

(event `self.ReceiveActorEndOverlap`
  (params (OtherActor :type "Actor Object Reference"))
  (bind _asbp_volcano_ball (cast `/Game/Blueprints/Volcanoball/BP_VolcanoBall` OtherActor))
  (`KismetArrayLibrary.Array_RemoveItem` (`self.Balls being touched`) _asbp_volcano_ball))

(event `self.ReceiveTick`
  (params (DeltaSeconds :type "Float (single-precision)"))
  (for _array_element (`self.Balls being touched`)
    (`PrimitiveComponent.AddImpulse` _array_element (* (`KismetMathLibrary.Normal` (`KismetMathLibrary.MakeVector` (.x (- (`self.K2_GetActorLocation` _array_element) (`self.K2_GetActorLocation`))) (.y (- (`self.K2_GetActorLocation` _array_element) (`self.K2_GetActorLocation`))))) (`self.Force`)) "None" true)))

(fn `UserConstructionScript`)