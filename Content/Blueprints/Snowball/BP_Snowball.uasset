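; BP_Snowball is a physics snowball hazard that kills any SnowballCharacter it hits.
; On BeginPlay it takes a random wait time from the SnowballGame game mode, and Tick keeps it hidden with its rigid body asleep until that time runs out.
; Other hits spawn a snow burst particle at the impact point, rate-limited by a cooldown that also counts down in Tick.
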(event `self.ReceiveBeginPlay`
  ;[1 1 1] Startup
  (bind _assnowball_game (cast `/Game/Blueprints/Snowball/SnowballGame` (`GameplayStatics.GetGameMode`)))
  (set `self.HideTime` (`/Game/Blueprints/Snowball/SnowballGame.Get Random Snowball Wait Time` _assnowball_game)))

(event `self.ReceiveTick`
  (params (DeltaSeconds :type "Float (single-precision)"))
  (bind _returnvalue (> (`self.HideTime`) 0.0))
  ;[1 1 1] Tick
  (`|ExecutionSequence`
    (:`then_0`
      (set `self.HideTime` (- (`self.HideTime`) DeltaSeconds))
      (`self.SetActorHiddenInGame` _returnvalue)
      (if _returnvalue
        (`PrimitiveComponent.PutRigidBodyToSleep` "None")
        (else
          (`PrimitiveComponent.WakeRigidBody` "None"))))
    (:`then_1`
      (set `self.Time Till Emit Again` (- (`self.Time Till Emit Again`) DeltaSeconds)))))

(event `self.ReceiveHit`
  (params (MyComp :type "PrimitiveComponent Object Reference") (Other :type "Actor Object Reference") (OtherComp :type "PrimitiveComponent Object Reference") (bSelfMoved :type Boolean) (HitLocation :type "Vector Structure") (HitNormal :type "Vector Structure") (NormalImpulse :type "Vector Structure") (Hit :type "HitResult Structure (by ref)"))
  (bind _assnowball_character (cast `/Game/Blueprints/Snowball/SnowballCharacter` Other)
    (:`then`
      (`/Game/Blueprints/Snowball/SnowballCharacter.Kill` _assnowball_character))
    (:`CastFailed`
      (if (< (`self.Time Till Emit Again`) 0.0)
        (`GameplayStatics.SpawnEmitterAtLocation` "/Game/Particles/P_SnowBurst.P_SnowBurst" HitLocation)
        (set `self.Time Till Emit Again` (`self.Time Between Particle Emits`))))))

(fn `UserConstructionScript`)