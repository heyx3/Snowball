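; SnowballGame is a Blueprint that holds shared state for a snowball game: the spawn node list and the random wait timing.
; On BeginPlay it clears RespawnNodes and refills it with every BP_SnowballSpawnNode actor in the level.
; GetRandomSnowballWaitTime returns a random value between the minimum and maximum wait settings by lerping with a random float.
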(event `self.ReceiveBeginPlay`
  (`KismetArrayLibrary.Array_Clear` (`self.Respawn Nodes`))
  (bind _outactors (`GameplayStatics.GetAllActorsOfClass` "/Game/Blueprints/BP_SnowballSpawnNode.BP_SnowballSpawnNode_C"))
  (for _array_element _outactors
    (`KismetArrayLibrary.Array_Add` (`self.Respawn Nodes`) _array_element)))

(fn `Get Random Snowball Wait Time`
  (returns (`Wait Time` :type "Float (double-precision)"))
  (return (`KismetMathLibrary.Lerp` (`self.Min Snowball Wait Time`) (`self.Max Snowball Wait Time`) (`KismetMathLibrary.RandomFloat`))))

(fn `UserConstructionScript`)